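; BP_PointSpawner fills the level with a grid of BP_Point actors when play begins.
; BeginPlay calls SpawnPoints, whose nested loops step through an 80 by 80 lattice at 100-unit spacing, at zero height in world space rather than relative to the spawner.
; Each spawn uses DontSpawnIfColliding, so points are left out wherever existing geometry or actors block them.
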(event EventBeginPlay
  (CallFunction|SpawnPoints))

(fn ConstructionScript)

(fn SpawnPoints
  (for _index (range 0 79)
    (LocalVariables|SetLocX (- (LocalVariables|GetLocX) 1e+02))
    (LocalVariables|SetLocY 3.95e+03)
    (for _index_2 (range 0 79)
      (Game|SpawnActorfromClass "/Game/_Game/Prop/Point/BP_Point.BP_Point_C" (Math|Conversions|ToTransform(Vector) (Math|Vector|MakeVector (LocalVariables|GetLocX) (LocalVariables|GetLocY) 0.0)) "DontSpawnIfColliding" "MultiplyWithRoot" 0 0)
      (LocalVariables|SetLocY (- (LocalVariables|GetLocY) 1e+02)))))