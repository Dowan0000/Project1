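; Fence placement preview that shows with red and green materials whether the fence can spawn and whether its ends meet other fences.
; Left and right SphereCollision overlaps with BP_Fence turn that end's sphere green, and red on exit.
; SpawnSphere overlaps with any other actor clear CanSpawn and redden the three cylinders.
; Any such end overlap restores both without counting remaining overlaps, and both events print debug strings.
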(event OnComponentBeginOverlap(SphereCollision_Left)
  (params (OverlappedComponent :type Primitive%20Component%20Object%20Reference) (OtherActor :type Actor%20Object%20Reference) (OtherComp :type Primitive%20Component%20Object%20Reference) (OtherBodyIndex :type Integer) (bFromSweep :type Boolean) (SweepResult :type Hit%20Result%20Structure%20%28by%20ref%29))
  (Utilities|Casting|CastToBP_Fence OtherActor)
  (Rendering|Material|SetMaterial (Variables|Default|GetSphere_Left) 0 "/Game/_Game/Prop/Fence/M_SphereCollision_Green.M_SphereCollision_Green"))

(event OnComponentBeginOverlap(SphereCollision_Right)
  (params (OverlappedComponent :type Primitive%20Component%20Object%20Reference) (OtherActor :type Actor%20Object%20Reference) (OtherComp :type Primitive%20Component%20Object%20Reference) (OtherBodyIndex :type Integer) (bFromSweep :type Boolean) (SweepResult :type Hit%20Result%20Structure%20%28by%20ref%29))
  (Utilities|Casting|CastToBP_Fence OtherActor)
  (Rendering|Material|SetMaterial (Variables|Default|GetSphere_Right) 0 "/Game/_Game/Prop/Fence/M_SphereCollision_Green.M_SphereCollision_Green"))

(event OnComponentEndOverlap(SphereCollision_Left)
  (params (OverlappedComponent :type Primitive%20Component%20Object%20Reference) (OtherActor :type Actor%20Object%20Reference) (OtherComp :type Primitive%20Component%20Object%20Reference) (OtherBodyIndex :type Integer))
  (Utilities|Casting|CastToBP_Fence OtherActor)
  (Rendering|Material|SetMaterial (Variables|Default|GetSphere_Left) 0 "/Game/_Game/Prop/Fence/M_SphereCollision_Red.M_SphereCollision_Red"))

(event OnComponentEndOverlap(SphereCollision_Right)
  (params (OverlappedComponent :type Primitive%20Component%20Object%20Reference) (OtherActor :type Actor%20Object%20Reference) (OtherComp :type Primitive%20Component%20Object%20Reference) (OtherBodyIndex :type Integer))
  (Utilities|Casting|CastToBP_Fence OtherActor)
  (Rendering|Material|SetMaterial (Variables|Default|GetSphere_Right) 0 "/Game/_Game/Prop/Fence/M_SphereCollision_Red.M_SphereCollision_Red"))

(event OnComponentBeginOverlap(SpawnSphere_Left)
  (params (OverlappedComponent :type Primitive%20Component%20Object%20Reference) (OtherActor :type Actor%20Object%20Reference) (OtherComp :type Primitive%20Component%20Object%20Reference) (OtherBodyIndex :type Integer) (bFromSweep :type Boolean) (SweepResult :type Hit%20Result%20Structure%20%28by%20ref%29))
  (if (!= OtherActor self)
    (Development|PrintString (Utilities|String|Append "BeginOverlap : " (Utilities|GetDisplayName OtherActor)))
    (Rendering|Material|SetMaterial (Variables|Default|GetCylinder_Top) 0 "/Game/_Game/Prop/Fence/M_SphereCollision_Red.M_SphereCollision_Red")
    (Variables|Default|SetbCanSpawn false)))

(event OnComponentEndOverlap(SpawnSphere_Left)
  (params (OverlappedComponent :type Primitive%20Component%20Object%20Reference) (OtherActor :type Actor%20Object%20Reference) (OtherComp :type Primitive%20Component%20Object%20Reference) (OtherBodyIndex :type Integer))
  (if (!= OtherActor self)
    (Development|PrintString "EndOverlap")
    (Rendering|Material|SetMaterial (Variables|Default|GetCylinder_Top) 0 "/Game/_Game/Prop/Fence/M_SphereCollision_Green.M_SphereCollision_Green")
    (Variables|Default|SetbCanSpawn true)))

(event OnComponentBeginOverlap(SpawnSphere_Right)
  (params (OverlappedComponent :type Primitive%20Component%20Object%20Reference) (OtherActor :type Actor%20Object%20Reference) (OtherComp :type Primitive%20Component%20Object%20Reference) (OtherBodyIndex :type Integer) (bFromSweep :type Boolean) (SweepResult :type Hit%20Result%20Structure%20%28by%20ref%29))
  (if (!= OtherActor self)
    (Development|PrintString (Utilities|String|Append "BeginOverlap : " (Utilities|GetDisplayName OtherActor)))
    (Rendering|Material|SetMaterial (Variables|Default|GetCylinder_Top) 0 "/Game/_Game/Prop/Fence/M_SphereCollision_Red.M_SphereCollision_Red")
    (Variables|Default|SetbCanSpawn false)))

(event OnComponentEndOverlap(SpawnSphere_Right)
  (params (OverlappedComponent :type Primitive%20Component%20Object%20Reference) (OtherActor :type Actor%20Object%20Reference) (OtherComp :type Primitive%20Component%20Object%20Reference) (OtherBodyIndex :type Integer))
  (if (!= OtherActor self)
    (Development|PrintString "EndOverlap")
    (Rendering|Material|SetMaterial (Variables|Default|GetCylinder_Top) 0 "/Game/_Game/Prop/Fence/M_SphereCollision_Green.M_SphereCollision_Green")
    (Variables|Default|SetbCanSpawn true)))

(event EventBeginPlay
  (Variables|Default|SetStartLocation (Transformation|GetActorLocation)))

(fn ConstructionScript)