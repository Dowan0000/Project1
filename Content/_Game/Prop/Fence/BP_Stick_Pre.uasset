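; Placement preview actor for a bamboo fence stick, showing whether the stick can be spawned at its current spot.
; Tick checks the bottom sphere for other overlapping actors, setting CanSpawn and a red or green material.
; SpawnConnectStick creates a connecting-stick preview at the raised midpoint toward another location, which SetConnectStick_Pre repositions and DestroyStick_Pre removes along with itself.
; Overlap events are empty, their former logic left disconnected.
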(event OnComponentBeginOverlap(Sphere)
  (params (OverlappedComponent :type Primitive%20Component%20Object%20Reference) (OtherActor :type Actor%20Object%20Reference) (OtherComp :type Primitive%20Component%20Object%20Reference) (OtherBodyIndex :type Integer) (bFromSweep :type Boolean) (SweepResult :type Hit%20Result%20Structure%20%28by%20ref%29)))

(event OnComponentEndOverlap(Sphere)
  (params (OverlappedComponent :type Primitive%20Component%20Object%20Reference) (OtherActor :type Actor%20Object%20Reference) (OtherComp :type Primitive%20Component%20Object%20Reference) (OtherBodyIndex :type Integer)))

(event OnComponentBeginOverlap(Sphere_Bottom)
  (params (OverlappedComponent :type Primitive%20Component%20Object%20Reference) (OtherActor :type Actor%20Object%20Reference) (OtherComp :type Primitive%20Component%20Object%20Reference) (OtherBodyIndex :type Integer) (bFromSweep :type Boolean) (SweepResult :type Hit%20Result%20Structure%20%28by%20ref%29)))

(event OnComponentEndOverlap(Sphere_Bottom)
  (params (OverlappedComponent :type Primitive%20Component%20Object%20Reference) (OtherActor :type Actor%20Object%20Reference) (OtherComp :type Primitive%20Component%20Object%20Reference) (OtherBodyIndex :type Integer)))

(event Custom|Set%20ConnectStick_Pre
  (bind _returnvalue (Transformation|GetActorLocation))
  (bind _other_location (Variables|Default|GetOther%20Location))
  (bind _bp_connectstick_pre (Variables|Default|GetBP_ConnectStick_Pre))
  (bind _returnvalue_2 (+ _returnvalue _other_location))
  (bind _returnvalue_3 (/ _returnvalue_2 2.0))
  ;[1 1 1] 수정
  (Utilities|IsValid _bp_connectstick_pre
    (:Is%20Valid
      (Transformation|SetActorTransform _bp_connectstick_pre (Math|Transform|MakeTransform (Math|Vector|MakeVector (.x _returnvalue_3) (.y _returnvalue_3) (+ (.z _returnvalue_3) 1e+02)) (Math|Rotator|FindLookatRotation (Transformation|GetActorLocation) (Variables|Default|GetOther%20Location)) "1.000000,1.000000,1.000000")))))

(event Custom|Destroy%20Stick_Pre
  (bind _bp_connectstick_pre (Variables|Default|GetBP_ConnectStick_Pre))
  (Utilities|IsValid _bp_connectstick_pre
    (:Is%20Valid
      (Actor|DestroyActor _bp_connectstick_pre))
    (:Is%20Not%20Valid
      _))
  (Actor|DestroyActor))

(event EventBeginPlay
  (Variables|Default|SetStartLocation (Transformation|GetActorLocation)))

(event EventTick
  (params (DeltaSeconds :type Float%20%28single-precision%29))
  (Variables|Default|SetbHasOverlappingActor false)
  (bind _array_element (Utilities|Array|ForEachLoopwithBreak (Collision|GetOverlappingActors (Variables|Default|GetSphere_Bottom) "/Script/Engine.Actor" :!class /Script/Engine.PrimitiveComponent) :!label _label)
    (:LoopBody
      (if (!= _array_element self)
        (Variables|Default|SetbHasOverlappingActor true)
        (goto _label Break)))
    (:Completed
      (if (Variables|Default|GetbHasOverlappingActor)
        (Rendering|Material|SetMaterial (Variables|Default|GetS_Bamboo_Stick_ud4pccafa_lod3_Var1) 0 "/Game/_Game/Prop/Fence/M_SphereCollision_Red.M_SphereCollision_Red")
        (Variables|Default|SetbCanSpawn false)
        (else
          (Rendering|Material|SetMaterial (Variables|Default|GetS_Bamboo_Stick_ud4pccafa_lod3_Var1) 0 "/Game/_Game/Prop/Fence/M_SphereCollision_Green.M_SphereCollision_Green")
          (Variables|Default|SetbCanSpawn true))))))

(fn ConstructionScript)

(fn SpawnConnectStick
  (params (Other%20Location :type Vector))
  (bind _returnvalue (Transformation|GetActorLocation))
  (bind _returnvalue_2 (+ _returnvalue Other%20Location))
  (bind _returnvalue_3 (/ _returnvalue_2 2.0))
  (Variables|Default|SetOther%20Location Other%20Location)
  (bind _returnvalue_4 (Game|SpawnActorfromClass "/Game/_Game/Prop/Fence/BP_ConnectStick_Pre.BP_ConnectStick_Pre_C" (Math|Transform|MakeTransform (Math|Vector|MakeVector (.x _returnvalue_3) (.y _returnvalue_3) (+ (.z _returnvalue_3) 1e+02)) (Math|Rotator|FindLookatRotation (Transformation|GetActorLocation) Other%20Location) "1.000000,1.000000,1.000000") "AdjustIfPossibleButAlwaysSpawn" "MultiplyWithRoot" 0 0))
  (Variables|Default|SetBP_ConnectStick_Pre _returnvalue_4))